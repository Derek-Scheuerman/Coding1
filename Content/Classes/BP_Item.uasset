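; BP_Item is an item actor, either a weapon or tool, that rolls its stats and strikes an enemy at BeginPlay.
; Constructor sets damage by type and replaces the "Excal" name with a random one from that type's list.
; After a short delay, Attack subtracts scaled damage from a found BP_Enemy's health, with on-screen debug prints.
; A Timeline also shifts the item's Z position each update.
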(event `self.ReceiveBeginPlay`
  (bind _item (`self.Item`))
  (bind (_returnvalue_x _returnvalue_y _returnvalue_z) (`KismetMathLibrary.BreakVector` (`SceneComponent.K2_GetComponentLocation` _item)))
  (`|ExecutionSequence`
    (:`then_0`
      (`self.Constructor`)
      (`KismetSystemLibrary.PrintString` (`KismetStringLibrary.Concat_StrStr` "Name: " (`self.Name`) " \nMy damage: " (`KismetStringLibrary.Conv_IntToString` (`self.Damage`))) true true (struct :`G` 0.66 :`B` 1.0 :`A` 1.0) 10.0)
      (`KismetSystemLibrary.Delay` 0.2)
      (bind _returnvalue (`GameplayStatics.GetActorOfClass` "/Game/Blueprints/Enemies/BP_Enemy.BP_Enemy_C"))
      (`self.Attack` _returnvalue)
      (bind _asbp_enemy (cast `/Game/Blueprints/Enemies/BP_Enemy` _returnvalue))
      (`KismetSystemLibrary.PrintString` (`KismetStringLibrary.Conv_DoubleToString` (`/Game/Blueprints/Enemies/BP_Enemy.Health` _asbp_enemy)) true true (struct :`G` 0.66 :`B` 1.0 :`A` 1.0) 10.0))
    (:`then_1`
      (bind (_direction _newtrack_0) (`Timeline|Timeline`)
        (:`Update`
          (`SceneComponent.K2_SetRelativeLocation` _item (`KismetMathLibrary.MakeVector` _returnvalue_x _returnvalue_y (+ _returnvalue_z (* _newtrack_0 10.0))) false false))))))

(fn `Attack`
  (params (Enemy :type "/Game/Blueprints/Enemies/BP_Enemy Object Reference"))
  (set `/Game/Blueprints/Enemies/BP_Enemy.Health` (- (`/Game/Blueprints/Enemies/BP_Enemy.Health` Enemy) (* (`KismetMathLibrary.Conv_IntToDouble` (`self.Damage`)) 0.01)) Enemy))

(fn `Constructor`
  (bind _weaponnames (`self.WeaponNames`))
  (bind _toolsnames (`self.ToolsNames`))
  (switch `/Game/Classes/ItemType` (`self.Type`)
    (:`NewEnumerator0`
      (set `self.Damage` (`KismetMathLibrary.RandomIntegerInRange` 3 6))
      (if (`KismetStringLibrary.EqualEqual_StrStr` (`self.Name`) "Excal")
        (`KismetArrayLibrary.Array_Shuffle` _weaponnames)
        (set `self.Name` (`|GetArrayItem` _weaponnames))))
    (:`NewEnumerator1`
      (set `self.Damage` 1)
      (if (`KismetStringLibrary.EqualEqual_StrStr` (`self.Name`) "Excal")
        (`KismetArrayLibrary.Array_Shuffle` _toolsnames)
        (set `self.Name` (`|GetArrayItem` _toolsnames))))))

(fn `UserConstructionScript`)