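; BP_Enemy_Spawner populates the level with BP_Enemy actors and spawns a new wave once none remain.
; On BeginPlay it gathers all BP_Enemy_Spawn_Location actors and prints their count as debug output.
; SpawnEnemies gives each location a weighted 70% chance to spawn an enemy at its transform, then starts CheckEnemyCount after each spawn.
; CheckEnemyCount polls the live enemy count through a self-calling Delay loop and calls SpawnEnemies when it reaches zero.
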(event `self.ReceiveBeginPlay`
  (bind _outactors (`GameplayStatics.GetAllActorsOfClass` "/Game/Blueprints/Enemies/BP_Enemy_Spawn_Location.BP_Enemy_Spawn_Location_C"))
  (`KismetSystemLibrary.PrintString` (`KismetStringLibrary.Concat_StrStr` "There are: " (`KismetStringLibrary.Conv_IntToString` (`KismetArrayLibrary.Array_Length` _outactors)) " total spawn locations") true true (struct :`G` 0.66 :`B` 1.0 :`A` 1.0) 10.0)
  (`self.Spawn Enemies`))

(event `Spawn Enemies`
  (for _array_element (stale `self.ReceiveBeginPlay` _outactors)
    (if (`KismetMathLibrary.RandomBoolWithWeight` 0.7)
      (`|SpawnActorFromClass` "/Game/Blueprints/Enemies/BP_Enemy.BP_Enemy_C" (`self.GetTransform` _array_element) "Undefined" "MultiplyWithRoot" null null)
      (`self.CheckEnemyCount`))))

(event `CheckEnemyCount`
  (bind _outactors (`GameplayStatics.GetAllActorsOfClass` "/Game/Blueprints/Enemies/BP_Enemy.BP_Enemy_C"))
  (if (not (> (`KismetArrayLibrary.Array_Length` _outactors) 0))
    (`self.Spawn Enemies`))
  (`KismetSystemLibrary.Delay` 0.2)
  (`self.CheckEnemyCount`))

(fn `UserConstructionScript`)