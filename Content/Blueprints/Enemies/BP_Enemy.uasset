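; Enemy actor that dies when its hitbox touches a BP_KillBox.
; The overlap drives Health negative and prints a red scream on screen.
; From BeginPlay, CheckHealth re-calls itself after a short delay instead of using Tick, destroying the actor once Health drops below zero.
; An unconnected chain, which never runs, would lerp the actor's transform toward a look-at of the player.
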(event `self.ReceiveBeginPlay`
  (`self.CheckHealth`))

(event `CheckHealth`
  (`KismetSystemLibrary.Delay` 0.2)
  (if (>= (`self.Health`) 0.0)
    (`self.CheckHealth`)
    (else
      (`self.K2_DestroyActor`))))

(event `self.Hitbox.OnComponentBeginOverlap`
  (params (OverlappedComponent :type "PrimitiveComponent Object Reference") (OtherActor :type "Actor Object Reference") (OtherComp :type "PrimitiveComponent Object Reference") (OtherBodyIndex :type Integer) (bFromSweep :type Boolean) (SweepResult :type "HitResult Structure (by ref)"))
  (cast `/Game/Blueprints/Objects/BP_KillBox` OtherActor)
  (set `self.Health` -1.0)
  (`KismetSystemLibrary.PrintString` "AHHHHHHHHHHHHHHHHHHHHHHHHHHHHHHHHHHHHHHHHHHHHHHHH" true true (struct :`R` 0.579167 :`A` 1.0) 10.0))

(fn `UserConstructionScript`)