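; BP_CoolBox is an actor that endlessly spawns BP_Key actors just above its Cube component.
; On BeginPlay it prints debug messages with its name, the cube's location and the raised spawn point.
; It then spawns a randomly but uniformly scaled key, waits SpawnDelay and wires back to the spawn node, forming a Delay-based loop with no exit.
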(event `self.ReceiveBeginPlay`
  (bind _returnvalue (`SceneComponent.K2_GetComponentLocation` (`self.Cube`)))
  (bind _returnvalue_2 (+ _returnvalue (0.0 0.0 100.0)))
  (`KismetSystemLibrary.PrintString` (`KismetStringLibrary.Concat_StrStr` (`KismetSystemLibrary.GetDisplayName` self) " exists!") true true (struct :`G` 0.66 :`B` 1.0 :`A` 1.0) 10.0) ; This is like cout\nThis sends text to the screen
  (`KismetSystemLibrary.PrintString` (`KismetStringLibrary.Conv_VectorToString` _returnvalue) true true (struct :`R` 1.0 :`B` 0.004811 :`A` 1.0) 10.0) ; This is like cout\nThis sends text to the screen
  (`KismetSystemLibrary.PrintString` (`KismetStringLibrary.Conv_VectorToString` _returnvalue_2) true true (struct :`G` 0.242635 :`B` 1.0 :`A` 1.0) 10.0) ; This is like cout\nThis sends text to the screen
  (`|SpawnActorFromClass` "/Game/Blueprints/BP_Key.BP_Key_C" (`KismetMathLibrary.MakeTransform` _returnvalue_2 (struct) (`KismetMathLibrary.Conv_DoubleToVector` (`KismetMathLibrary.RandomFloatInRange` 0.1 1.0))) "Undefined" "MultiplyWithRoot" null null :!label _label)
  (`KismetSystemLibrary.Delay` (`self.Spawn Delay`))
  (goto _label))

(fn `UserConstructionScript`)