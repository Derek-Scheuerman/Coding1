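; BP_KillBox is an actor with a physics-driven cube that resets to its starting spot after falling out of the level.
; BeginPlay stores the cube's world location and also triggers one reset after a long delay.
; Tick watches for the cube dropping below a fixed height, then, after a short delay, teleports the actor to the origin and briefly switches physics simulation off and on.
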(event `self.ReceiveBeginPlay`
  (bind _cube (`self.Cube`))
  (set `self.OriginLoc` (`SceneComponent.K2_GetComponentLocation` (`self.Cube`)))
  (`KismetSystemLibrary.Delay` 100.0)
  (`self.K2_SetActorLocation` (`self.OriginLoc`) false true :!label _label)
  (`PrimitiveComponent.SetSimulatePhysics` _cube false)
  (`KismetSystemLibrary.Delay` 0.2)
  (`PrimitiveComponent.SetSimulatePhysics` _cube true))

(event `self.ReceiveTick`
  (params (DeltaSeconds :type "Float (single-precision)"))
  (bind (_returnvalue_x _returnvalue_y _returnvalue_z) (`KismetMathLibrary.BreakVector` (`SceneComponent.K2_GetComponentLocation` (`self.Cube`))))
  (if (< _returnvalue_z -100.0)
    (`KismetSystemLibrary.Delay` 0.5)
    (goto _label)))

(fn `UserConstructionScript`)