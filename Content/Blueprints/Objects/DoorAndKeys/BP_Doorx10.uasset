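; BP_Doorx10 is a key-locked door that opens by destroying itself when the third-person character has enough white keys.
; A hit on its Cube casts the other actor to BP_ThirdPersonCharacter and checks TotalKeys for at least five, despite the x10 name.
; Success zeroes the whole count rather than subtracting five, then prints a total five below that.
; Otherwise, an on-screen message states the requirement.
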(event `self.Cube.OnComponentHit`
  (params (HitComponent :type "PrimitiveComponent Object Reference") (OtherActor :type "Actor Object Reference") (OtherComp :type "PrimitiveComponent Object Reference") (NormalImpulse :type "Vector Structure") (Hit :type "HitResult Structure (by ref)"))
  (bind _asbp_third_person_character (cast `/Game/ThirdPerson/Blueprints/BP_ThirdPersonCharacter` OtherActor))
  (bind _totalkeys (`/Game/ThirdPerson/Blueprints/BP_ThirdPersonCharacter.TotalKeys` _asbp_third_person_character))
  (if (> _totalkeys 4)
    (set `/Game/ThirdPerson/Blueprints/BP_ThirdPersonCharacter.TotalKeys` 0 _asbp_third_person_character)
    (`self.K2_DestroyActor`) ; open door
    (`KismetSystemLibrary.PrintString` (`KismetStringLibrary.Concat_StrStr` "Opened Door! \n \nRemoved 5 white keys \nTotal Keys =" (`KismetStringLibrary.Conv_IntToString` (- _totalkeys 5))))
    (else
      (`KismetSystemLibrary.PrintString` "You need 5 White Keys!" true true (struct :`R` 0.939261 :`G` 0.940237 :`B` 1.0 :`A` 1.0)))))

(fn `UserConstructionScript`)